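; BP_Mother is a team's "Mother" character, whose death ends the match in favor of the opposing team.
; Incoming damage passes through Damage to DamageMulti, which lowers health (체력) and updates the nameplate widget.
; On first reaching zero health it ragdolls the mesh and calls GameEnding on ALS_GameMode_SP, deriving the winner from 호스트팀 (host team).
; MotherSpawn, also called by SetSit, restores health, animation and collision.
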(event `Damage`
  (params (B :type "Float (double-precision)"))
  (`self.DamageMulti` B))

(event `DamageMulti`
  (params (B :type "Float (double-precision)"))
  (bind _mesh (`self.Mesh`))
  (bind _output_get (set `self.체력` (- (`self.체력`) B)))
  (bind _asw_nameplate (cast `/Game/UI/Indicators/W_Nameplate` (`WidgetComponent.GetWidget` (`self.HealthBar`))))
  (`/Game/UI/Indicators/W_Nameplate.SetHealth` _asw_nameplate (/ _output_get 100.0))
  (if (`self.사망`)
    _
    (elif (<= (`self.체력`) 0.0)
      (set `self.사망` true)
      (`PrimitiveComponent.SetSimulatePhysics` _mesh true)
      (`SkeletalMeshComponent.SetAnimationMode` _mesh "AnimationCustomMode")
      (`PrimitiveComponent.SetCollisionProfileName` _mesh "Ragdoll" true)
      (bind _asals_game_mode_sp (cast `/Game/AdvancedLocomotionV4/Blueprints/GameModes/ALS_GameMode_SP` (`GameplayStatics.GetGameMode`)))
      (`/Game/AdvancedLocomotionV4/Blueprints/GameModes/ALS_GameMode_SP.GameEnding` _asals_game_mode_sp (not (`self.호스트팀`)) true))))

(event `self.ReceiveAnyDamage`
  (params (Damage :type "Float (single-precision)") (DamageType :type "DamageType Object Reference") (InstigatedBy :type "Controller Object Reference") (DamageCauser :type "Actor Object Reference"))
  (`self.Damage` Damage))

(event `MotherSpawn`
  (bind _mesh (`self.Mesh`))
  (set `self.체력` 100.0)
  (set `self.사망` false)
  (bind _asw_nameplate (cast `/Game/UI/Indicators/W_Nameplate` (`WidgetComponent.GetWidget` (`self.HealthBar`))))
  (`/Game/UI/Indicators/W_Nameplate.SetHealth` _asw_nameplate 1.0)
  (`PrimitiveComponent.SetSimulatePhysics` _mesh false)
  (`SkeletalMeshComponent.SetAnimationMode` _mesh "AnimationBlueprint")
  (`PrimitiveComponent.SetCollisionProfileName` _mesh "CharacterMesh" true))

(event `SetSit`
  (`self.MotherSpawn`))

(fn `UserConstructionScript`)